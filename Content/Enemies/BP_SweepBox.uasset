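; BP_SweepBox is an enemy hazard volume that arms after a short delay, damages the first-person character, then expires.
; On BeginPlay it waits, swaps the cube to an active material, enables damage and sets its lifespan.
; Box overlap events cache the player and track whether they are inside.
; While armed and overlapped, Tick applies fixed damage every frame, so total damage depends on frame rate.
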(event OnComponentBeginOverlap(Box)
  (params (OverlappedComponent :type Primitive%20Component%20Object%20Reference) (OtherActor :type Actor%20Object%20Reference) (OtherComp :type Primitive%20Component%20Object%20Reference) (OtherBodyIndex :type Integer) (bFromSweep :type Boolean) (SweepResult :type Hit%20Result%20Structure%20%28by%20ref%29))
  (bind _asbp_first_person_character (Utilities|Casting|CastToBP_FirstPersonCharacter OtherActor))
  (Variables|Default|SetOverlapping true))

(event OnComponentEndOverlap(Box)
  (params (OverlappedComponent :type Primitive%20Component%20Object%20Reference) (OtherActor :type Actor%20Object%20Reference) (OtherComp :type Primitive%20Component%20Object%20Reference) (OtherBodyIndex :type Integer))
  (Utilities|Casting|CastToBP_FirstPersonCharacter OtherActor)
  (Variables|Default|SetOverlapping false))

(event EventBeginPlay
  (Utilities|FlowControl|Delay 1.0)
  (Rendering|Material|SetMaterial (Variables|Default|GetCube) 0 "/Game/Enemies/M_SweepActive.M_SweepActive")
  (Variables|Default|SetCanDamage true)
  (Actor|SetLifeSpan 2.5))

(event EventTick
  (params (DeltaSeconds :type Float%20%28single-precision%29))
  (if (and (Variables|Default|GetCanDamage) (Variables|Default|GetOverlapping))
    (Game|Damage|ApplyDamage (stale OnComponentBeginOverlap(Box) _asbp_first_person_character) 1.0 0 0)))

(fn ConstructionScript)
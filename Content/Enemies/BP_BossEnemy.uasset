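; Boss enemy that picks attacks through the AI blackboard's BossAttack key and quits the game when destroyed.
; Pawn sensing flags the player as seen and selects Shove at close range unless roaming; otherwise attacks are randomised between Sweep, LongRange and Roam.
; Attack events spawn sweep, shove or projectile actors, with the laser tracking the player by debug-drawn traces while charging.
; Damage reduces health and destroys the boss at zero.
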(event OnSeePawn(PawnSensing)
  (params (Pawn :type Pawn%20Object%20Reference))
  (bind _returnvalue (Transformation|GetActorLocation))
  (bind _returnvalue_2 (Utilities|Name|MakeLiteralName "BossAttack"))
  (bind _self self)
  (bind _returnvalue_3 (AI|GetAIController _self))
  (bind _returnvalue_4 (AI|GetBlackboard _returnvalue_3))
  ;[0.5724 0.6015 1] Pawn Sensing
  (bind _asbp_first_person_character (Utilities|Casting|CastToBP_FirstPersonCharacter Pawn))
  (AI|Components|Blackboard|SetValueasBool (AI|GetBlackboard (AI|GetAIController self)) (Utilities|Name|MakeLiteralName "SeenPlayer") true)
  (if (Math|Boolean|ANDBoolean (and (>= (- (.x _returnvalue) (.x (Transformation|GetActorLocation _asbp_first_person_character))) -3e+02) (<= (- (.x _returnvalue) (.x (Transformation|GetActorLocation _asbp_first_person_character))) 3e+02)) (and (>= (- (.y _returnvalue) (.y (Transformation|GetActorLocation _asbp_first_person_character))) -3e+02) (<= (- (.y _returnvalue) (.y (Transformation|GetActorLocation _asbp_first_person_character))) 3e+02)) (!= (Class|BlackboardComponent|GetValueasName _returnvalue_4 _returnvalue_2) "Roam"))
    (Class|BlackboardComponent|SetValueasName _returnvalue_4 _returnvalue_2 "Shove")))

(event Custom|SweepAttack
  ;[1 0.9123 0.5649] Sweep Attack
  (Transformation|SetActorRotation (Math|Rotator|FindRelativeLookatRotation (Math|Conversions|ToTransform(Vector) (Transformation|GetActorLocation)) (Transformation|GetActorLocation (stale OnSeePawn(PawnSensing) _asbp_first_person_character))))
  (Game|SpawnActorfromClass "/Game/Enemies/BP_SweepBox.BP_SweepBox_C" (Math|Conversions|ToTransform(Vector) (Math|Vector|MakeVector (.x (Transformation|GetActorLocation (stale OnSeePawn(PawnSensing) _asbp_first_person_character))) (.y (Transformation|GetActorLocation (stale OnSeePawn(PawnSensing) _asbp_first_person_character))) 5e+01)) "Undefined" "MultiplyWithRoot" 0 0)
  (CallFunction|RandomiseAttack))

(event Custom|ShoveAttack
  (Game|SpawnActorfromClass "/Game/Enemies/BP_ShoveRadius.BP_ShoveRadius_C" (Math|Conversions|ToTransform(Vector) (Transformation|GetActorLocation)) "Undefined" "MultiplyWithRoot" 0 0)
  (Utilities|FlowControl|Delay 6.0)
  (CallFunction|RandomiseAttack))

(event Custom|StartLaserCharge
  ;[0.4597 1 0.4957] Long Range Attack (laser)
  (Variables|Default|SetChargingBeam true)
  (Utilities|Time|SetTimerbyEvent (delegate Custom|FireLaser) 2.5))

(event Custom|FireLaser
  (bind _projspawn (Variables|Default|GetProjSpawn))
  ;[0.4597 1 0.4957] Long Range Attack (laser)
  (Variables|Default|SetChargingBeam false)
  (Transformation|SetActorRotation (Math|Rotator|FindRelativeLookatRotation (Math|Conversions|ToTransform(Vector) (Transformation|GetActorLocation)) (Transformation|GetActorLocation (stale OnSeePawn(PawnSensing) _asbp_first_person_character))))
  (Variables|Default|SetChargeFinalLocation (Transformation|GetActorLocation (stale OnSeePawn(PawnSensing) _asbp_first_person_character)))
  (Collision|LineTraceForObjects (Transformation|GetWorldLocation _projspawn) (Transformation|GetActorLocation (stale OnSeePawn(PawnSensing) _asbp_first_person_character)) (Utilities|Array|MakeArray "ObjectTypeQuery3") false 0 "ForDuration")
  (Utilities|FlowControl|Delay 1.0)
  (Game|SpawnActorfromClass "/Game/Enemies/BP_EnemyProjectile.BP_EnemyProjectile_C" (Transformation|GetWorldTransform _projspawn) "Undefined" "MultiplyWithRoot" 0 0)
  (CallFunction|RandomiseAttack))

(event Custom|RandomiseAttack
  (bind _returnvalue (Utilities|Name|MakeLiteralName "BossAttack"))
  (bind _self self)
  (bind _returnvalue_2 (AI|GetAIController _self))
  (bind _returnvalue_3 (AI|GetBlackboard _returnvalue_2))
  (switch int (Math|Random|RandomIntegerinRange 0 2)
    (:0
      (Class|BlackboardComponent|SetValueasName _returnvalue_3 _returnvalue "Sweep"))
    (:1
      (Class|BlackboardComponent|SetValueasName _returnvalue_3 _returnvalue "LongRange"))
    (:2
      (Class|BlackboardComponent|SetValueasName _returnvalue_3 _returnvalue "Roam"))))

(event EventBeginPlay)

(event Collision|EventActorBeginOverlap
  (params (OtherActor :type Actor%20Object%20Reference)))

(event Game|Damage|EventAnyDamage
  (params (Damage :type Float%20%28single-precision%29) (DamageType :type Damage%20Type%20Object%20Reference) (InstigatedBy :type Controller%20Object%20Reference) (DamageCauser :type Actor%20Object%20Reference))
  (bind _output_get (Variables|Default|SetHealth (- (Variables|Default|GetHealth) Damage)))
  (Development|PrintString (Utilities|String|Append "BossHealth is:" (Utilities|String|ToString(Float) _output_get)))
  (if (<= _output_get 0.0)
    (Actor|DestroyActor)))

(event EventTick
  (params (DeltaSeconds :type Float%20%28single-precision%29))
  (bind _returnvalue (Utilities|Name|MakeLiteralName "BossAttack"))
  (bind _self self)
  (bind _returnvalue_2 (AI|GetAIController _self))
  (bind _returnvalue_3 (AI|GetBlackboard _returnvalue_2))
  (bind _returnvalue_4 (Class|BlackboardComponent|GetValueasName _returnvalue_3 _returnvalue))
  (if (Math|Boolean|ANDBoolean (== _returnvalue_4 "") (ScalableFloat|GetValueasBool _returnvalue_3 (Utilities|Name|MakeLiteralName "SeenPlayer")) (!= _returnvalue_4 "Shove"))
    (CallFunction|RandomiseAttack)
    (elif (Variables|Default|GetChargingBeam)
      (Transformation|SetActorRotation (Math|Rotator|FindRelativeLookatRotation (Math|Conversions|ToTransform(Vector) (Transformation|GetActorLocation)) (Transformation|GetActorLocation (stale OnSeePawn(PawnSensing) _asbp_first_person_character))))
      (Collision|LineTraceForObjects (Transformation|GetWorldLocation (Variables|Default|GetProjSpawn)) (Transformation|GetActorLocation (stale OnSeePawn(PawnSensing) _asbp_first_person_character)) (Utilities|Array|MakeArray "ObjectTypeQuery3") false 0 "ForDuration" true "(R=1.000000,G=0.000000,B=0.000000,A=1.000000)" "(R=0.000000,G=1.000000,B=0.000000,A=1.000000)" 0.1)
      (elif (Variables|Default|GetShoving)
        (Transformation|SetActorRotation (Math|Rotator|FindRelativeLookatRotation (Math|Conversions|ToTransform(Vector) (Transformation|GetActorLocation)) (Transformation|GetActorLocation (stale OnSeePawn(PawnSensing) _asbp_first_person_character))))))))

(event EventDestroyed
  (Game|QuitGame 0 "Quit" false))

(fn ConstructionScript)